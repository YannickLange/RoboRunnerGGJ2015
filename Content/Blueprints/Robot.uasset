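; Robot Blueprint that shows a colored laser beam running from the actor's location to its aim end point.
; The construction script creates a dynamic material instance from the laser particle component.
; Each tick updates the beam's source and target points and pushes the element color, set to red on BeginPlay, into that material's Color parameter.
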(event EventBeginPlay
  (|CallParentFunction)
  (Variables|Default|SetElementColor (Math|Conversions|ToColor(LinearColor) (Math|Color|MakeColor 1.0 0.0 0.0))))

(event EventTick
  (params (DeltaSeconds :type Float%20%28single-precision%29))
  (|CallParentFunction DeltaSeconds)
  (Class|ParticleSystemComponent|SetBeamTargetPoint 0 (Variables|Default|GetAimEndLocation))
  (Class|ParticleSystemComponent|SetBeamSourcePoint 0 (Transformation|GetActorLocation))
  (Rendering|Material|SetVectorParameterValue (Variables|Default|GetLaserDynamicMaterial) "Color" (Math|Conversions|ToLinearColor(Color) (Variables|Default|GetElementColor)) :!class /Script/Engine.MaterialInstanceDynamic))

(fn ConstructionScript
  (bind _returnvalue (Rendering|Material|CreateDynamicMaterialInstance (Variables|Default|GetLaserParticle) 0 0 :!class /Script/Engine.PrimitiveComponent))
  (Variables|Default|SetLaserDynamicMaterial _returnvalue))