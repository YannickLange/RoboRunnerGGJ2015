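; Pickup orb that Monster or Robot actors can take, respawning with a random green, blue or orange color after a short cooldown.
; PickUpAvailable returns whether the orb was active and, for those classes, deactivates it, toggles the mesh's visibility and starts the EndCooldown timer.
; EndCooldown rerolls OrbColor, reactivates the orb and toggles visibility again, while a looping timer applies the color to the GreenGlow light.
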(event EventBeginPlay
  (|CallParentFunction)
  (CallFunction|EndCooldown)
  (Utilities|Time|SetTimerbyFunctionName 0 "Update" 0.2 true))

(fn ConstructionScript)

(fn EndCooldown
  (bind _returnvalue (CallFunction|GetRandomColor))
  (Variables|Default|SetorbColor _returnvalue)
  (Variables|Default|SetActive true)
  (Rendering|ToggleVisibility (Variables|Default|GetStaticMesh1) true))

(fn PickUpAvailable
  (params (NewParam :type Object%20Object%20Reference))
  (bind _returnvalue (Utilities|GetClass NewParam))
  (Variables|Default|SetPlaceholderActive (Variables|Default|GetActive))
  (if (and (or (Utilities|ClassIsChildOf _returnvalue "/Script/RoboRunners.Monster") (Utilities|ClassIsChildOf _returnvalue "/Script/RoboRunners.Robot")) (Variables|Default|GetPlaceholderActive))
    (Utilities|Time|SetTimerbyFunctionName 0 "EndCooldown" 5.0)
    (Variables|Default|SetActive false)
    (Rendering|ToggleVisibility (Variables|Default|GetStaticMesh1) true))
  (return (Variables|Default|GetPlaceholderActive)))

(fn GetRandomColor
  (switch int (Math|Random|RandomIntegerinRange 0 2)
    (:0
      (LocalVariables|SetReturnColor (Math|Color|MakeColor 0.3 1.0 0.3)))
    (:1
      (LocalVariables|SetReturnColor (Math|Color|MakeColor 0.0 0.4 1.0)))
    (:2
      (LocalVariables|SetReturnColor (Math|Color|MakeColor 1.0 0.4 0.2))))
  (return (LocalVariables|GetReturnColor)))

(fn Update
  (Rendering|Components|Light|SetLightColor (Variables|Default|GetGreenGlow) (Variables|Default|GetorbColor)))