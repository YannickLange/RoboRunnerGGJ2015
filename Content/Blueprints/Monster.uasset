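; Monster actor that absorbs orb colors from pick-ups and sends the game to the menu when its health runs out.
; Overlapping an available Pick-Up copies its orb color to ElementColor, which Tick applies to the light every frame.
; Tick also checks health and calls SwitchToMenu on GameControl.
; GetRobotSpawn returns a random position from nearby overlapping RobotSpawn actors, appending to a list it never clears.
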(event EventActorBeginOverlap
  (params (OtherActor :type Actor%20Object%20Reference))
  (bind _aspick__up (Utilities|Casting|CastToPick-Up OtherActor))
  (bind _newparam (Default|PickUpAvailable _aspick__up self))
  (if _newparam
    (Variables|Default|SetElementColor (Math|Conversions|ToColor(LinearColor) (Variables|/Game/Blueprints/Pick-Up.Pick-Up_C|GetorbColor _aspick__up)))))

(event EventTick
  (params (DeltaSeconds :type Float%20%28single-precision%29))
  (|CallParentFunction DeltaSeconds)
  (Rendering|Components|Light|SetLightColor (Variables|Default|GetLight) (Math|Conversions|ToLinearColor(Color) (Variables|Default|GetElementColor)))
  (if (<= (Variables|Default|GetHealth) 0.0)
    (bind _outactors (Actor|GetAllActorsOfClass 0 "/Game/Blueprints/GameControl.GameControl_C"))
    (bind _asgame_control (Utilities|Casting|CastToGameControl (Utilities|Array|Get(acopy) _outactors)))
    (Default|SwitchtoMenu _asgame_control)))

(fn ConstructionScript)

(fn GetRobotSpawn
  (bind _possiblepositions (LocalVariables|GetPossiblePositions))
  (LocalVariables|SetMonsterPosition (Transformation|GetActorLocation self))
  (for _array_element (Collision|GetOverlappingActors "/Game/Blueprints/RobotSpawn.RobotSpawn_C" :!class /Script/Engine.PrimitiveComponent)
    (if (< (Math|Vector|VectorLength (- (Transformation|GetActorLocation _array_element) (LocalVariables|GetMonsterPosition))) 1e+04)
      (Utilities|Array|Add (LocalVariables|GetPossiblePositions) (Transformation|GetActorLocation _array_element))))
  (return (Utilities|Array|Get(acopy) _possiblepositions (Math|Random|RandomInteger (Utilities|Array|Length _possiblepositions)))))