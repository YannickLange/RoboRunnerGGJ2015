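; MazeExit is the maze's exit actor, which sends the game back to the menu when a Monster overlaps it.
; The overlap event checks the other actor's class against Monster, then calls SwitchToMenu on the first GameControl found in the level.
; Open and Close hide and show two components by toggling visibility only, without changing collision or gating the overlap check.
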(event EventActorBeginOverlap
  (params (OtherActor :type Actor%20Object%20Reference))
  (if (Utilities|ClassIsChildOf (Utilities|GetClass OtherActor) "/Script/RoboRunners.Monster")
    (bind _outactors (Actor|GetAllActorsOfClass "/Game/Blueprints/GameControl.GameControl_C"))
    (bind _asgame_control (Utilities|Casting|CastToGameControl (Utilities|Array|Get(acopy) _outactors)))
    (Default|SwitchtoMenu _asgame_control)))

(fn ConstructionScript)

(fn Open
  (Rendering|SetVisibility false false)
  (Rendering|SetVisibility false false))

(fn Close
  (Rendering|SetVisibility true false)
  (Rendering|SetVisibility true false))