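; GameControl switches the game between menu and a local multiplayer match of one Monster against three Robots, starting in menu on BeginPlay.
; SwitchToMenu destroys all Monsters and Robots and gives player 0 a FloatingCamera.
; SwitchToGame spawns a Monster at a random MonsterSpawn for player 0, then half-scale Robots at Monster-supplied locations for players 1 to 3.
; An InGame flag blocks repeated match starts.
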(event EventBeginPlay
  (Variables|Default|SetInGame true)
  (CallFunction|SwitchtoMenu))

(fn ConstructionScript)

(fn SwitchtoMenu
  (bind _outactors (Actor|GetAllActorsOfClass "/Script/RoboRunners.Monster"))
  (Actor|DestroyActor _outactors)
  (bind _outactors_2 (Actor|GetAllActorsOfClass "/Script/RoboRunners.Robot"))
  (Actor|DestroyActor _outactors_2)
  (bind _outactors_3 (Actor|GetAllActorsOfClass "/Game/Blueprints/FloatingCamera.FloatingCamera_C"))
  (Pawn|Possess (Game|GetPlayerController 0) (Utilities|Array|Get(acopy) _outactors_3))
  (Variables|Default|SetInGame false))

(fn SwitchtoGame
  (if (not (Variables|Default|GetInGame))
    (bind _outactors (Actor|GetAllActorsOfClass "/Game/Blueprints/MonsterSpawn.MonsterSpawn_C"))
    (bind _returnvalue (Game|SpawnActorfromClass "/Game/Blueprints/Monster.Monster_C" (Math|Transform|MakeTransform (Transformation|GetActorLocation (Utilities|Array|Get(acopy) _outactors (Math|Random|RandomInteger (Utilities|Array|Length _outactors)))) "0, 0, 0" "1.000000,1.000000,1.000000") true 0))
    (Pawn|Possess (Game|GetPlayerController 0) _returnvalue)
    (bind _asmonster (Utilities|Casting|CastToMonster _returnvalue))
    (for _index (range 1 3)
      (bind _spawnposition (Default|GetRobotSpawn _asmonster))
      (Development|PrintString (Utilities|String|ToString(Vector) _spawnposition))
      (bind _returnvalue_2 (Game|SpawnActorfromClass "/Game/Blueprints/Robot.Robot_C" (Math|Transform|MakeTransform _spawnposition "0, 0, 0" "0.500000,0.500000,0.500000") true 0))
      (Pawn|Possess (Game|GetPlayerController _index) _returnvalue_2))
    (Variables|Default|SetInGame true)))